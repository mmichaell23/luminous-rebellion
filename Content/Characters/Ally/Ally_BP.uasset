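; Allied character that walks along the X axis each tick, fires on enemies and dies when health runs out.
; An enemy entering DetectEnemy starts an endless delayed loop spawning Ally_Bullet_BP at the Projectile transform, with that enemy as Owner.
; Enemy bullets hitting the Damage component apply fixed damage and are destroyed.
; AnyDamage clamps health, updates the widget health bar and destroys the ally shortly after zero.
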(event `self.ReceiveAnyDamage`
  (params (Damage :type "Float (single-precision)") (DamageType :type "DamageType Object Reference") (InstigatedBy :type "Controller Object Reference") (DamageCauser :type "Actor Object Reference"))
  (bind _returnvalue (`KismetMathLibrary.Clamp` (- (`self.Current Health`) (`KismetMathLibrary.FTrunc` Damage)) 0 (`self.Max Health`)))
  ;[1 1 1] Health Control
  (set `self.Current Health` _returnvalue)
  (`/Game/Characters/Ally/Ally_HealthBar.UpdateHealth` (`self.Ally Health Bar`) _returnvalue)
  (if (== 0 (`self.Current Health`))
    (`KismetSystemLibrary.Delay` 0.5)
    (`self.K2_DestroyActor`)))

(event `self.Damage.OnComponentBeginOverlap`
  (params (OverlappedComponent :type "PrimitiveComponent Object Reference") (OtherActor :type "Actor Object Reference") (OtherComp :type "PrimitiveComponent Object Reference") (OtherBodyIndex :type Integer) (bFromSweep :type Boolean) (SweepResult :type "HitResult Structure (by ref)"))
  ;[1 1 1] Attack
  (bind _asenemy_bullet_bp (cast `/Game/Characters/Enemy/Enemy_Bullet_BP` OtherActor))
  (`GameplayStatics.ApplyDamage` self 20.0)
  (`self.K2_DestroyActor` _asenemy_bullet_bp))

(event `self.Detect Enemy.OnComponentBeginOverlap`
  (params (OverlappedComponent :type "PrimitiveComponent Object Reference") (OtherActor :type "Actor Object Reference") (OtherComp :type "PrimitiveComponent Object Reference") (OtherBodyIndex :type Integer) (bFromSweep :type Boolean) (SweepResult :type "HitResult Structure (by ref)"))
  ;[1 1 1] Bullet Projectile
  (bind _asenemy_bp (cast `/Game/Characters/Enemy/Enemy_BP` OtherActor))
  (`self.Direction`)
  (`KismetSystemLibrary.Delay` 1.0 :!label _label)
  (`|SpawnActorFromClass` "/Game/Characters/Ally/Ally_Bullet_BP.Ally_Bullet_BP_C" (`SceneComponent.K2_GetComponentToWorld` (`self.Projectile`)) "Undefined" "OverrideRootScale" _asenemy_bp null)
  (goto _label))

(event `Direction`
  ;[1 1 1] Movement
  (`SceneComponent.K2_SetRelativeRotation` (`self.Sprite`) (`KismetMathLibrary.MakeRotator` 0.0 0.0 (`KismetMathLibrary.SelectFloat` 180.0 0.0 (`self.IsMovingRight`))) false false)
  (`self.AddMovementInput` (`KismetMathLibrary.SelectVector` (-1.0 0.0 0.0) (1.0 0.0 0.0) (`self.IsMovingRight`))))

(event `self.ReceiveBeginPlay`
  ;[1 1 1] Health
  (bind _asally_health_bar (cast `/Game/Characters/Ally/Ally_HealthBar` (`WidgetComponent.GetUserWidgetObject` (`self.Widget`))))
  (bind _output_get (set `self.Ally Health Bar` _asally_health_bar))
  (set `/Game/Characters/Ally/Ally_HealthBar.Current_Health` (`self.Current Health`) _output_get)
  (set `/Game/Characters/Ally/Ally_HealthBar.MaxHealth` (`self.Max Health`) _output_get))

(event `self.ReceiveTick`
  (params (DeltaSeconds :type "Float (single-precision)"))
  (`self.Direction`))

(fn `UserConstructionScript`)