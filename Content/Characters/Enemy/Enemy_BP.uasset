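; Side-scrolling enemy character that walks along X, shoots, and rewards the player with health when killed.
; Tick drives movement and sprite flipping from IsMovingRight.
; Player overlap with DetectEnemy starts an endless one-second delay loop spawning Enemy_Bullet_BP at Projectile.
; Ally bullets hitting the Damage component apply fixed damage, updating the widget health bar; at zero it destroys itself and heals BP_Lelouch unless already at 100.
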(event `self.ReceiveAnyDamage`
  (params (Damage :type "Float (single-precision)") (DamageType :type "DamageType Object Reference") (InstigatedBy :type "Controller Object Reference") (DamageCauser :type "Actor Object Reference"))
  (bind _health (`/Game/Characters/Protagonist/BP_Lelouch.Health` (`self.Main Char`)))
  (bind _returnvalue (`KismetMathLibrary.Clamp` (- (`self.Current Health`) (`KismetMathLibrary.FTrunc` Damage)) 0 (`self.Max Health`)))
  ;[1 1 1] Health Control
  (set `self.Current Health` _returnvalue)
  (`/Game/Characters/Enemy/Enemy_HealthBar.UpdateHealth` (`self.Enemy Health Bar`) _returnvalue)
  (if (== 0 (`self.Current Health`))
    (`KismetSystemLibrary.Delay` 0.5)
    (`self.K2_DestroyActor`)
    (bind _asbp_lelouch (cast `/Game/Characters/Protagonist/BP_Lelouch` (`GameplayStatics.GetPlayerPawn` 0)))
    (bind _output_get (set `self.Main Char` _asbp_lelouch))
    (if (not (== 100.0 _health))
      (set `/Game/Characters/Protagonist/BP_Lelouch.Health` (+ _health 13.0) _output_get))))

(event `self.Damage.OnComponentBeginOverlap`
  (params (OverlappedComponent :type "PrimitiveComponent Object Reference") (OtherActor :type "Actor Object Reference") (OtherComp :type "PrimitiveComponent Object Reference") (OtherBodyIndex :type Integer) (bFromSweep :type Boolean) (SweepResult :type "HitResult Structure (by ref)"))
  ;[1 1 1] Attack
  (bind _asally_bullet_bp (cast `/Game/Characters/Ally/Ally_Bullet_BP` OtherActor))
  (`GameplayStatics.ApplyDamage` self 20.0 null null "/Script/Engine.DamageType")
  (`self.K2_DestroyActor` _asally_bullet_bp))

(event `self.Detect Enemy.OnComponentBeginOverlap`
  (params (OverlappedComponent :type "PrimitiveComponent Object Reference") (OtherActor :type "Actor Object Reference") (OtherComp :type "PrimitiveComponent Object Reference") (OtherBodyIndex :type Integer) (bFromSweep :type Boolean) (SweepResult :type "HitResult Structure (by ref)"))
  ;[1 1 1] Bullet Projectile
  (bind _asbp_lelouch (cast `/Game/Characters/Protagonist/BP_Lelouch` OtherActor))
  (`self.Direction`)
  (`KismetSystemLibrary.Delay` 1.0 :!label _label)
  (`|SpawnActorFromClass` "/Game/Characters/Enemy/Enemy_Bullet_BP.Enemy_Bullet_BP_C" (`SceneComponent.K2_GetComponentToWorld` (`self.Projectile`)) "Undefined" "OverrideRootScale" _asbp_lelouch null)
  (goto _label))

(event `Direction`
  ;[1 1 1] Movement
  (`SceneComponent.K2_SetRelativeRotation` (`self.Sprite`) (`KismetMathLibrary.MakeRotator` 0.0 0.0 (`KismetMathLibrary.SelectFloat` 180.0 0.0 (`self.IsMovingRight`))) false false)
  (`self.AddMovementInput` (`KismetMathLibrary.SelectVector` (1.0 0.0 0.0) (-1.0 0.0 0.0) (`self.IsMovingRight`))))

(event `self.ReceiveTick`
  (params (DeltaSeconds :type "Float (single-precision)"))
  ;[1 1 1] Movement
  (`self.Direction`))

(event `self.ReceiveBeginPlay`
  ;[1 1 1] Health
  (bind _asenemy_health_bar (cast `/Game/Characters/Enemy/Enemy_HealthBar` (`WidgetComponent.GetUserWidgetObject` (`self.Widget`))))
  (bind _output_get (set `self.Enemy Health Bar` _asenemy_health_bar))
  (set `/Game/Characters/Enemy/Enemy_HealthBar.Current_Health` (`self.Current Health`) _output_get)
  (set `/Game/Characters/Enemy/Enemy_HealthBar.MaxHealth` (`self.Max Health`) _output_get))

(fn `UserConstructionScript`)